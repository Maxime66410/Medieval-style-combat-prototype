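; BP_Character is a Blueprint in the Medieval Market pack that lets the player delete fruit actors through key presses.
; G clears the Spawn flag and stores the last index of FruitArray in Ultimo.
; Each X press destroys the actor at Ultimo and steps the index back, working from the end of the array without removing entries or checking bounds.
; The graphs shown never fill FruitArray.
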(event EventBeginPlay)

(event Collision|EventActorBeginOverlap
  (params (OtherActor :type Actor%20Object%20Reference)))

(event EventTick
  (params (DeltaSeconds :type Float%20%28single-precision%29)))

(event Input|KeyboardEvents|G
  (params (Key :type Key%20Structure))
  (:Pressed
    (Variables|Default|SetbSpawn false)
    (Variables|Default|SetUltimo (Utilities|Array|LastIndex (Variables|Default|GetFruitArray)))))

(event Input|KeyboardEvents|X
  (params (Key :type Key%20Structure))
  (:Pressed
    (Actor|DestroyActor (Utilities|Array|Get(acopy) (Variables|Default|GetFruitArray) (Variables|Default|GetUltimo)))
    (Variables|Default|SetUltimo (- (Variables|Default|GetUltimo) 1))))

(fn ConstructionScript)