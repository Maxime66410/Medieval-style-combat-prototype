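; BP_Spawner is an actor that repeatedly spawns a chosen fruit class at its own location.
; On BeginPlay it casts the player pawn to BP_Character, then loops with a 0.2 second delay while that character's Spawn flag is true.
; Each spawned actor is added to the character's FruitArray.
; The loop ends once Spawn reads false, with nothing to restart it.
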(event EventBeginPlay
  (bind _asbp_character (Utilities|Casting|CastToBP_Character (Game|Player|GetPlayerPawn 0)))
  (if (Variables|/Game/Content/Model/MedievalMarketPack/Blueprints/BP_Character.BP_Character_C|GetbSpawn _asbp_character) :!label _label
    (Utilities|FlowControl|Delay 0.2)
    (bind _returnvalue (Game|SpawnActorfromClass (Variables|Default|GetFruitToSpawn) (Math|Conversions|ToTransform(Vector) (Transformation|GetActorLocation self)) "AlwaysSpawn" 0 0))
    (Utilities|Array|Add (Variables|/Game/Content/Model/MedievalMarketPack/Blueprints/BP_Character.BP_Character_C|GetFruitArray _asbp_character) _returnvalue)
    (goto _label)))

(fn ConstructionScript)