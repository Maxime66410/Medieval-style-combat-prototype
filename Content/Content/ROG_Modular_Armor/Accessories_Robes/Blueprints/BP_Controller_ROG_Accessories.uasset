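; Player controller for the ROG Modular Armor accessories content that shows an on-screen accessories selector widget.
; BeginPlay creates BPW_Accessories_Selector, adds it to the viewport and calls ToggleSelectorWidget, which Tab also triggers.
; The toggle flips the selector canvas visibility and mouse cursor together.
; Its input-mode branch is fixed to true, so it always sets Game and UI focused on the canvas, never Game Only.
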(event EventBeginPlay
  (bind _returnvalue (UserInterface|CreateWidget "/Game/Content/ROG_Modular_Armor/Accessories_Robes/Blueprints/BPW_Accessories_Selector.BPW_Accessories_Selector_C" self))
  (Variables|Default|SetAccessoriesSelector _returnvalue)
  (UserInterface|Viewport|AddtoViewport (Variables|Default|GetAccessoriesSelector) 0)
  (CallFunction|ToggleSelectorWidget))

(event Input|KeyboardEvents|Tab
  (params (Key :type Key%20Structure))
  (:Pressed
    (CallFunction|ToggleSelectorWidget)))

(fn ConstructionScript)

(fn ToggleSelectorWidget
  (Variables|Default|SetShowingSelectorWidget (not (Variables|Default|GetShowingSelectorWidget)))
  (Widget|SetVisibility (Variables|/Game/Content/ROG_Modular_Armor/Accessories_Robes/Blueprints/BPW_Accessories_Selector.BPW_Accessories_Selector_C|GetCanvasPanel_Selector (Variables|Default|GetAccessoriesSelector)) (select (Variables|Default|GetShowingSelectorWidget) "Visible" "Hidden"))
  (Variables|Default|SetbShowMouseCursor (Variables|Default|GetShowingSelectorWidget))
  (if true
    (Input|SetInputModeGameandUI self (Variables|/Game/Content/ROG_Modular_Armor/Accessories_Robes/Blueprints/BPW_Accessories_Selector.BPW_Accessories_Selector_C|GetCanvasPanel_Selector (Variables|Default|GetAccessoriesSelector)) "DoNotLock" true)
    (else
      (Input|SetInputModeGameOnly self))))