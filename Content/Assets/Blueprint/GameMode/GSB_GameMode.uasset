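; Multiplayer game mode that runs the match clock, team scoring and start conditions for FFA, TDM or CTF, read from the session settings.
; One-second re-arming timers refresh the player name list, tick the countdown to game over and wait for at least two players.
; Once the match starts, each player gets an independently random team, and AddPoints scores for either team only during live, non-FFA play.
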(event Custom|PlayerList
  ;[1 1 1] Update Players List
  (Utilities|Array|Clear (Variables|Default|GetListPlayers))
  (bind _outactors (Actor|GetAllActorsOfClass "/Game/Assets/Blueprint/Player/BP_Player.BP_Player_C"))
  (for _array_element _outactors
    (Utilities|Array|AddUnique (Variables|Default|GetListPlayers) (Variables|/Game/Assets/Blueprint/Player/BP_Player.BP_Player_C|GetPlayerName _array_element)))
  (Utilities|Time|SetTimerbyEvent (delegate Custom|PlayerList) 1.0))

(event Custom|CheckIfGameCanStart
  ;[1 1 1] Game Can Start ?
  (if (>= (Utilities|Array|Length (Variables|Default|GetListPlayers)) 2)
    (Variables|Default|SetGameIsStart? true)
    (CallFunction|RandomTeam)
    (else
      (Utilities|Time|SetTimerbyEvent (delegate Custom|CheckIfGameCanStart) 1.0))))

(event Custom|RandomTeam
  ;[1 1 1] Random Team On Start
  (bind _outactors (Actor|GetAllActorsOfClass "/Game/Assets/Blueprint/Player/BP_Player.BP_Player_C"))
  (for _array_element _outactors
    (Variables|/Game/Assets/Blueprint/Player/BP_Player.BP_Player_C|SetE_Team _array_element (.OutItem (Utilities|Array|Random (Utilities|Array|MakeArray "NewEnumerator0" "NewEnumerator1"))))))

(event Custom|TimeSystem
  ;[1 1 1] Time System
  (if (Variables|Default|GetGameIsStart?)
    (if (not (Variables|Default|GetGameIsFinish?))
      (if (!= (Variables|Default|GetSeconds) 0)
        (Math|Integer|DecrementInt (Variables|Default|GetSeconds)
          (:%20%20
            _))
        (elif (!= (Variables|Default|GetMinutes) 0)
          (Math|Integer|DecrementInt (Variables|Default|GetMinutes)
            (:%20%20
              (Variables|Default|SetSeconds 60)))
          (else
            (Variables|Default|SetGameIsFinish? true))))
      (Utilities|Time|SetTimerbyEvent (delegate Custom|TimeSystem) 1.0)
      (else
        (Utilities|Time|SetTimerbyEvent (delegate Custom|TimeSystem) 1.0 :!label _label)))
    (else
      (goto _label))))

(event Custom|AddPoints
  (params (Teams :type TeamsClass%20Enum :default "NewEnumerator0"))
  (if (Variables|Default|GetGameIsStart?)
    (if (not (Variables|Default|GetGameIsFinish?))
      (if (Utilities|Enum|NotEqual(Enum) (Variables|Default|GetGameMode) "NewEnumerator0")
        (switch Utilities|FlowControl|Switch|SwitchonTeamsClass Teams
          (:NewEnumerator0
            (Utilities|Array|SetArrayElem (Variables|Default|GetPointSystem) 0 (+ (Utilities|Array|Get(acopy) (Variables|Default|GetPointSystem)) 1)))
          (:NewEnumerator1
            (Utilities|Array|SetArrayElem (Variables|Default|GetPointSystem) 1 (+ (Utilities|Array|Get(acopy) (Variables|Default|GetPointSystem) 1) 1))))))))

(event EventBeginPlay
  (bind _extrasettings (Class|AdvancedSessionsLibrary|GetSessionSettings)
    (:OnSuccess
      (bind _settingvalue (Class|AdvancedSessionsLibrary|GetSessionPropertyString _extrasettings "GameMode")
        (:Found
          (switch string _settingvalue
            (:FFA
              (Variables|Default|SetGameMode "NewEnumerator0"))
            (:TDM
              (Variables|Default|SetGameMode "NewEnumerator1"))
            (:CTF
              (Variables|Default|SetGameMode "NewEnumerator2"))))))
    (:OnFailure
      (Variables|Default|SetGameMode "NewEnumerator0")))
  (CallFunction|PlayerList)
  (CallFunction|TimeSystem)
  (CallFunction|CheckifGameCanStart))

(fn ConstructionScript)