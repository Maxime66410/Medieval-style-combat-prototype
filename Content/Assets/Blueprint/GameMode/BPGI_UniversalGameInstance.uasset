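; Universal Game Instance that handles PlayFab account registration and email/password login for the game.
; PF_Register and PF_Login each take a caller reference, send the PlayFab client request and bind success and failure callbacks.
; The callbacks report back to that caller through RegisterSystemReceive or LoginSystemReceive, passing the result on success or setting an error message on failure.
; Registration uses the display name as the username too.
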(event Custom|PF_Register
  (params (DisplayName :type String) (Email :type String) (PassWord :type String) (INSTANCE :type UI%20Main%20Menu%20Object%20Reference))
  ;[0.9845 1 0.2634] Register System
  (|RegisterPlayFabUser (Utilities|Struct|MakeClientRegisterPlayFabUserRequest 0 DisplayName Email "" 0 PassWord "" false DisplayName) (delegate Custom|OnRegister) (delegate Custom|OnFailureRegister)))

(event Custom|OnRegister
  (params (result :type Client%20Register%20Play%20Fab%20User%20Result%20Structure) (customData :type Object%20Object%20Reference))
  ;[0.9845 1 0.2634] Register System
  (Default|RegisterSystemReceive (stale Custom|PF_Register INSTANCE) true result))

(event Custom|OnFailureRegister
  (params (error :type Play%20Fab%20Error%20Structure) (customData :type Object%20Object%20Reference))
  ;[0.9845 1 0.2634] Register System
  (Default|SetMessageError (stale Custom|PF_Register INSTANCE) (Utilities|Text|ToText(String) (.errordetails error)))
  (Default|RegisterSystemReceive (stale Custom|PF_Register INSTANCE) false))

(event Custom|PF_Login
  (params (Email :type String) (Password :type String) (INSTANCED :type UI%20Main%20Menu%20Object%20Reference))
  ;[0.1931 0.3173 1] Login System
  (|LoginwithEmailAddress (Utilities|Struct|MakeClientLoginWithEmailAddressRequest 0 Email 0 Password) (delegate Custom|OnLogin) (delegate Custom|OnFailedLogin)))

(event Custom|OnLogin
  (params (result :type Client%20Login%20Result%20Structure) (customData :type Object%20Object%20Reference))
  ;[0.1931 0.3173 1] Login System
  (Default|LoginSystemReceive (stale Custom|PF_Login INSTANCED) true result))

(event Custom|OnFailedLogin
  (params (error :type Play%20Fab%20Error%20Structure) (customData :type Object%20Object%20Reference))
  ;[0.1931 0.3173 1] Login System
  (Default|SetMessageError (stale Custom|PF_Login INSTANCED) (Utilities|Text|ToText(String) (.errormessage error)))
  (Default|LoginSystemReceive (stale Custom|PF_Login INSTANCED) false))