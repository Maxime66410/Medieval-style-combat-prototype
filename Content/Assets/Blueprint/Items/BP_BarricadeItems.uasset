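; BP_BarricadeItems is a barricade item with a health pool that blocks, deals damage and can be destroyed.
; One second after BeginPlay, its static mesh is set to block all collision channels.
; Hits on the mesh apply a small point damage to the other actor, using the impact impulse as direction.
; Any damage the barricade receives reduces Health, and it destroys itself at zero or below.
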(event OnComponentHit(StaticMesh)
  (params (HitComponent :type Primitive%20Component%20Object%20Reference) (OtherActor :type Actor%20Object%20Reference) (OtherComp :type Primitive%20Component%20Object%20Reference) (NormalImpulse :type Vector :default "0, 0, 0") (Hit :type Hit%20Result%20Structure%20%28by%20ref%29))
  ;[1 1 1] Take Damage
  (Game|Damage|ApplyPointDamage OtherActor 1.0 NormalImpulse Hit))

(event EventBeginPlay
  (Utilities|FlowControl|Delay 1.0)
  (Collision|SetCollisionResponsetoAllChannels (Variables|Default|GetStaticMesh) "ECR_Block"))

(event Game|Damage|EventAnyDamage
  (params (Damage :type Float%20%28single-precision%29) (DamageType :type Damage%20Type%20Object%20Reference) (InstigatedBy :type Controller%20Object%20Reference) (DamageCauser :type Actor%20Object%20Reference))
  ;[1 1 1] Heal / Damage System
  (Variables|Default|SetHealth (- (Variables|Default|GetHealth) Damage))
  (if (<= (Variables|Default|GetHealth) 0.0)
    (Actor|DestroyActor)))

(fn ConstructionScript)