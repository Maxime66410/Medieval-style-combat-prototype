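; BP_OriflammeFlag is a destructible flag item that heals players standing inside its sphere zone.
; Sphere overlaps add and remove BP_Player actors in the PlayerHit list, matched by object name.
; From BeginPlay, a self-rescheduling timer calls the healing RPC on listed players every two seconds.
; Damage lowers its Health until it is destroyed, and a FlagIcon boolean picks the banner material after a short startup delay.
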(event OnComponentBeginOverlap(Sphere)
  (params (OverlappedComponent :type Primitive%20Component%20Object%20Reference) (OtherActor :type Actor%20Object%20Reference) (OtherComp :type Primitive%20Component%20Object%20Reference) (OtherBodyIndex :type Integer) (bFromSweep :type Boolean) (SweepResult :type Hit%20Result%20Structure%20%28by%20ref%29))
  ;[1 1 1] Collider Player Enter
  (bind _asbp_player (Utilities|Casting|CastToBP_Player OtherActor))
  (CallFunction|AddPlr _asbp_player))

(event OnComponentEndOverlap(Sphere)
  (params (OverlappedComponent :type Primitive%20Component%20Object%20Reference) (OtherActor :type Actor%20Object%20Reference) (OtherComp :type Primitive%20Component%20Object%20Reference) (OtherBodyIndex :type Integer))
  ;[1 1 1] Collider Player Exit
  (bind _asbp_player (Utilities|Casting|CastToBP_Player OtherActor))
  (CallFunction|RemovePlr _asbp_player))

(event Custom|HealPlayer
  ;[1 1 1] Heal Player If In Zone
  (for _array_element (Variables|Default|GetPlayerHit)
    (Default|RPCHealingPlayer _array_element 5.0))
  (Utilities|Time|SetTimerbyEvent (delegate Custom|HealPlayer) 2.0))

(event Custom|FlagIcon
  (bind _medieval_flag_plane_004 (Variables|Default|Getmedieval_flag_Plane_004))
  ;[1 1 1] Flag Mat
  (Utilities|FlowControl|Delay 0.08)
  (if (Variables|Default|GetFlagIcon?)
    (Rendering|Material|SetMaterial _medieval_flag_plane_004 0 "/Game/Assets/Models/Flag/M_flag_BPS.M_flag_BPS")
    (else
      (Rendering|Material|SetMaterial _medieval_flag_plane_004 0 "/Game/Assets/Models/Flag/M_flag_VDS.M_flag_VDS"))))

(event Game|Damage|EventAnyDamage
  (params (Damage :type Float%20%28single-precision%29) (DamageType :type Damage%20Type%20Object%20Reference) (InstigatedBy :type Controller%20Object%20Reference) (DamageCauser :type Actor%20Object%20Reference))
  ;[1 1 1] Heal / Damage System
  (Variables|Default|SetHealth (- (Variables|Default|GetHealth) Damage))
  (if (<= (Variables|Default|GetHealth) 0.0)
    (Actor|DestroyActor)))

(event EventBeginPlay
  (CallFunction|HealPlayer)
  (CallFunction|FlagIcon))

(fn ConstructionScript)

(fn AddPlr
  (params (Plr :type BP%20Player%20Object%20Reference))
  (bind _array_element (Utilities|Array|ForEachLoopwithBreak (Variables|Default|GetPlayerHit) :!label _label)
    (:LoopBody
      (if (Utilities|Enum|Equal(Enum) (Utilities|GetObjectName _array_element) (Utilities|GetObjectName Plr))
        (LocalVariables|SetIsNewPlayer? false)
        (goto _label Break)))
    (:Completed
      (if (LocalVariables|GetIsNewPlayer?)
        (Utilities|Array|AddUnique (Variables|Default|GetPlayerHit) Plr)))))

(fn RemovePlr
  (params (Plr :type BP%20Player%20Object%20Reference))
  (bind _array_element (Utilities|Array|ForEachLoopwithBreak (Variables|Default|GetPlayerHit) :!label _label)
    (:LoopBody
      (if (Utilities|Enum|Equal(Enum) (Utilities|GetObjectName _array_element) (Utilities|GetObjectName Plr))
        (Utilities|Array|RemoveItem (Variables|Default|GetPlayerHit) _array_element)
        (goto _label Break)))))