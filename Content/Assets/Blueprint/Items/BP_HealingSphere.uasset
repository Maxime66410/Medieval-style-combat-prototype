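; BP_HealingSphere is an actor that follows a referenced player and heals players who enter its sphere.
; Each Tick it moves to the capsule location of BPPlayers, and sphere overlaps with a BP_Player call Heal.
; Heal compares object names against PlayerHit, then calls RPCHealingPlayer with a fixed amount and records new players.
; IsNewPlayer is never reset to true here, so one repeat match blocks later heals.
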(event OnComponentBeginOverlap(Sphere)
  (params (OverlappedComponent :type Primitive%20Component%20Object%20Reference) (OtherActor :type Actor%20Object%20Reference) (OtherComp :type Primitive%20Component%20Object%20Reference) (OtherBodyIndex :type Integer) (bFromSweep :type Boolean) (SweepResult :type Hit%20Result%20Structure%20%28by%20ref%29))
  ;[1 1 1] Collider Player
  (bind _asbp_player (Utilities|Casting|CastToBP_Player OtherActor))
  (CallFunction|Heal _asbp_player))

(event EventTick
  (params (DeltaSeconds :type Float%20%28single-precision%29))
  (bind _bp_players (Variables|Default|GetBP_Players))
  ;[1 1 1] Follow Players
  (Utilities|IsValid _bp_players
    (:Is%20Valid
      (Transformation|SetActorLocation (Transformation|GetWorldLocation (Variables|/Script/Engine.Character|GetCapsuleComponent _bp_players)) false false))))

(fn ConstructionScript)

(fn Heal
  (params (Plr :type BP%20Player%20Object%20Reference))
  (bind _array_element (Utilities|Array|ForEachLoopwithBreak (Variables|Default|GetPlayerHit) :!label _label)
    (:LoopBody
      (if (Utilities|Enum|Equal(Enum) (Utilities|GetObjectName _array_element) (Utilities|GetObjectName Plr))
        (LocalVariables|SetIsNewPlayer? false)
        (goto _label Break)))
    (:Completed
      (if (LocalVariables|GetIsNewPlayer?)
        (Default|RPCHealingPlayer Plr 15.0)
        (Utilities|Array|AddUnique (Variables|Default|GetPlayerHit) Plr)))))