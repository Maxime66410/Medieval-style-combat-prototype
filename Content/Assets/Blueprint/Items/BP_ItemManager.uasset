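; BP_ItemManager is a world item actor that shows weapon and shield meshes for an item selected from a list.
; Shortly after BeginPlay it reads the selected entry and assigns its sword and shield meshes.
; An outer glow zone toggles custom depth on both meshes as BP_Player enters or leaves.
; Player overlap with TriggerBox only prints a pickup-attempt message, and GetItemName has no connected logic.
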(event OnComponentBeginOverlap(TriggerBox)
  (params (OverlappedComponent :type Primitive%20Component%20Object%20Reference) (OtherActor :type Actor%20Object%20Reference) (OtherComp :type Primitive%20Component%20Object%20Reference) (OtherBodyIndex :type Integer) (bFromSweep :type Boolean) (SweepResult :type Hit%20Result%20Structure%20%28by%20ref%29))
  (bind _asbp_player (Utilities|Casting|CastToBP_Player OtherActor))
  (Development|PrintString (Utilities|String|Append (Utilities|GetDisplayName _asbp_player) " Trying to take a " (Utilities|GetItemName))))

(event OnComponentBeginOverlap(ZoneEnabledGlow)
  (params (OverlappedComponent :type Primitive%20Component%20Object%20Reference) (OtherActor :type Actor%20Object%20Reference) (OtherComp :type Primitive%20Component%20Object%20Reference) (OtherBodyIndex :type Integer) (bFromSweep :type Boolean) (SweepResult :type Hit%20Result%20Structure%20%28by%20ref%29))
  (Utilities|Casting|CastToBP_Player OtherActor)
  (Rendering|SetRenderCustomDepth (Variables|Default|GetWeapon) true)
  (Rendering|SetRenderCustomDepth (Variables|Default|GetShield) true))

(event OnComponentEndOverlap(ZoneEnabledGlow)
  (params (OverlappedComponent :type Primitive%20Component%20Object%20Reference) (OtherActor :type Actor%20Object%20Reference) (OtherComp :type Primitive%20Component%20Object%20Reference) (OtherBodyIndex :type Integer))
  (Utilities|Casting|CastToBP_Player OtherActor)
  (Rendering|SetRenderCustomDepth (Variables|Default|GetWeapon) false)
  (Rendering|SetRenderCustomDepth (Variables|Default|GetShield) false))

(event EventBeginPlay
  (Utilities|FlowControl|Delay 0.05)
  (Variables|Default|SetItemToAdd (Utilities|Array|Get(acopy) (.list (Variables|Default|GetListOfItems)) (Variables|Default|GetSelectItems)))
  (Components|StaticMesh|SetStaticMesh (Variables|Default|GetWeapon) (.meshsword (Variables|Default|GetItemToAdd)))
  (Components|StaticMesh|SetStaticMesh (Variables|Default|GetShield) (.meshshield (Variables|Default|GetItemToAdd))))

(fn ConstructionScript)