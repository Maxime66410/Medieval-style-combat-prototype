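; Trigger-box zone that hurts players on entry, acting as a damage, dead or fire zone according to the selected value in its Type map.
; Damage zones apply light point damage and dead zones apply heavy damage to living players, while the fire zone is an empty stub.
; CheckHitPlayer tracks hit players by object name to avoid repeat hits, and any player leaving the box clears that list.
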(event OnComponentBeginOverlap(Box)
  (params (OverlappedComponent :type Primitive%20Component%20Object%20Reference) (OtherActor :type Actor%20Object%20Reference) (OtherComp :type Primitive%20Component%20Object%20Reference) (OtherBodyIndex :type Integer) (bFromSweep :type Boolean) (SweepResult :type Hit%20Result%20Structure%20%28by%20ref%29))
  ;[1 1 1] Enter on Box
  (bind _keys (Utilities|Map|Keys (Variables|Default|GetType)))
  (bind _array_element (Utilities|Array|ForEachLoopwithBreak _keys :!label _label)
    (:LoopBody
      (if (Utilities|Name|Equal(Name) (.Value (Utilities|Map|Find (Variables|Default|GetType) _array_element)) (Variables|Default|GetValueSelected))
        (switch int _array_element
          (:-1
            (CallFunction|DamageZone OtherActor)
            (goto _label Break))
          (:0
            (CallFunction|FireZone OtherActor)
            (goto _label Break))
          (:1
            (CallFunction|DeadZone OtherActor)
            (goto _label Break)))))))

(event OnComponentEndOverlap(Box)
  (params (OverlappedComponent :type Primitive%20Component%20Object%20Reference) (OtherActor :type Actor%20Object%20Reference) (OtherComp :type Primitive%20Component%20Object%20Reference) (OtherBodyIndex :type Integer))
  ;[1 1 1] Reset List Array
  (Utilities|Casting|CastToBP_Player OtherActor)
  (Utilities|ResetPlayerHit))

(event Custom|DamageZone
  (params (Actor :type Actor%20Object%20Reference))
  (bind _returnvalue (Transformation|GetActorLocation))
  ;[1 1 1] DamageZone
  (bind _isalreadyins (CallFunction|CheckHitPlayer Actor))
  (if _isalreadyins
    (Game|Damage|ApplyPointDamage Actor 1e+01 _returnvalue (Collision|MakeHitResult false false 0.0 0.0 _returnvalue "0, 0, 0" "0,0,1" "0,0,1" 0 0) 0 self)))

(event Custom|FireZone
  (params (Actor :type Actor%20Object%20Reference)))

(event Custom|DeadZone
  (params (Actor :type Actor%20Object%20Reference))
  (bind _returnvalue (Transformation|GetActorLocation))
  ;[1 1 1] DeadZone
  (bind _isalreadyins (CallFunction|CheckHitPlayer Actor))
  (if _isalreadyins
    (bind _asbp_player (Utilities|Casting|CastToBP_Player Actor)
      (:then
        (if (> (Variables|/Game/Assets/Blueprint/Player/BP_Player.BP_Player_C|GetHealth _asbp_player) 0.0)
          (Game|Damage|ApplyPointDamage Actor 1e+02 _returnvalue (Collision|MakeHitResult false false 0.0 0.0 _returnvalue "0, 0, 0" "0,0,1" "0,0,1" 0 0) 0 self :!label _label)))
      (:CastFailed
        (goto _label)))))

(fn ConstructionScript)

(fn CheckHitPlayer
  (params (B :type Object%20Object%20Reference))
  (bind _asbp_player (Utilities|Casting|CastToBP_Player B)
    (:then
      ;[1 0.3737 0.3538] Check Is Not Already Hit
      (bind _array_element (Utilities|Array|ForEachLoopwithBreak (Variables|Default|GetP_AttackTouchPlayer) :!label _label)
        (:LoopBody
          (if (Utilities|Enum|Equal(Enum) (Utilities|GetObjectName _array_element) (Utilities|GetObjectName _asbp_player))
            (LocalVariables|SetIsAlreadyIN false)
            (goto _label Break)))
        (:Completed
          (if (not (LocalVariables|GetIsAlreadyIN))
            (return (LocalVariables|GetIsAlreadyIN))
            (else
              (Utilities|Array|AddUnique (Variables|Default|GetP_AttackTouchPlayer) _asbp_player)
              (return (LocalVariables|GetIsAlreadyIN)))))))
    (:CastFailed
      (return (LocalVariables|GetIsAlreadyIN)))))